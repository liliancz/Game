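; BP_icetrap is an ice trap that damages and knocks back any Base_0 actor that hits its box.
; On a Box1 hit, it subtracts DamageCanDo from that actor's HealthCurrent.
; It then uses MoveComponentTo to shift the actor's capsule upward and toward negative X, regardless of approach direction.
; Finally, it tints its PaperFlipbook to half-transparent black, with no reset in the graph.
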(event OnComponentHit(Box1)
  (params (HitComponent :type Primitive%20Component%20Object%20Reference) (OtherActor :type Actor%20Object%20Reference) (OtherComp :type Primitive%20Component%20Object%20Reference) (NormalImpulse :type Vector :default "0, 0, 0") (Hit :type Hit%20Result%20Structure%20%28by%20ref%29))
  (bind _asbase_0 (Utilities|Casting|CastToBase_0 OtherActor))
  (Variables|/Game/BLUEPRINTS/Characters/Base_0.Base_0_C|SetHealth_current _asbase_0 (- (Variables|/Game/BLUEPRINTS/Characters/Base_0.Base_0_C|GetHealth_current _asbase_0) (Variables|Default|GetDamage_can_do)))
  (Components|MoveComponentTo (Variables|/Script/Engine.Character|GetCapsuleComponent _asbase_0) (Math|Vector|MakeVector (- (.x (Transformation|GetActorLocation _asbase_0)) 3e+01) 0.0 (+ (.z (Transformation|GetActorLocation _asbase_0)) 5e+01)) "0, 0, 0" false false 0.2 false)
  (Sprite|SetSpriteColor (Variables|Default|GetPaperFlipbook) "(R=0.000000,G=0.000000,B=0.000000,A=0.500000)"))

(fn ConstructionScript)