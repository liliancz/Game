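; Base character Blueprint that moves itself continuously along world +X every tick, as in an auto-runner, with Jump input for jumping.
; A Health function subtracts damage and returns the remaining percentage and a death flag.
; Health_check, also triggered by the Z key, applies fixed damage through it and only prints the result.
; Power_up is an empty stub.
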(event Custom|Health_check
  ;[1 1 1] Comment
  (bind (_health_percentage _isdeath_) (Character|Health 3e+01))
  (if _isdeath_
    (Development|PrintString "death")
    (else
      (Development|PrintString (Utilities|String|ToString(Float) _health_percentage)))))

(event Custom|Power_up)

(event EventTick
  (params (DeltaSeconds :type Float%20%28single-precision%29))
  ;[1 1 1] run >>
  (Utilities|FlowControl|Sequence
    (:then_0
      (Pawn|Input|AddMovementInput self "6.000000, 0, 0" 1.0 false))))

(event Input|ActionEvents|InputActionJump
  (params (Key :type Key%20Structure :default "None"))
  ;[1 1 1] JUMP= double jump
  (:Pressed
    (Character|Jump))
  (:Released
    (Character|StopJumping)))

(event Input|KeyboardEvents|Z
  (params (Key :type Key%20Structure :default "None"))
  ;[1 1 1] Comment
  (:Pressed
    (bind (_health_percentage _isdeath_) (Character|Health 3e+01))
    (if _isdeath_
      (Development|PrintString "death")
      (else
        (Development|PrintString (Utilities|String|ToString(Float) _health_percentage))))))

(event Input|KeyboardEvents|T
  (params (Key :type Key%20Structure :default "None")))

(fn ConstructionScript)

(fn Health
  (params (damage :type Float%20%28single-precision%29))
  (bind _output_get (Variables|Default|SetHealth_current (- (Variables|Default|GetHealth_current) damage)))
  (return (/ _output_get (Variables|Default|GetHealth_Max)) (<= _output_get 0.0)))